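; Single Japanese sliding door (fusuma) actor that the player slides open along world X by holding F nearby.
; BeginPlay caches the start position and player character, and F press and release toggle a held flag.
; While F is held within range, Tick nudges the door by a fixed, frame-rate-dependent step and clamps it at a maximum offset from the start.
; The door has no closing logic.
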(event `self.ReceiveBeginPlay`
  (bind _output_get (set `self.Pos` (`self.K2_GetActorLocation`)))
  (set `self.StartPos` _output_get)
  (set `self.Player` (`GameplayStatics.GetPlayerCharacter` 0)))

(event `Key|F`
  (params (Key :type "Key Structure"))
  (:`Pressed`
    (set `self.PressKey` true))
  (:`Released`
    (set `self.PressKey` false)))

(event `self.ReceiveTick`
  (params (DeltaSeconds :type "Float (single-precision)"))
  (bind (_pos_x _pos_y _pos_z) (`KismetMathLibrary.BreakVector` (`self.Pos`)))
  (bind _pos_x_2 (`KismetMathLibrary.BreakVector` (`self.Pos`)))
  (bind _startpos_x (`KismetMathLibrary.BreakVector` (`self.StartPos`)))
  (if (`self.PressKey`)
    (if (< (`KismetMathLibrary.VSize` (- (`self.K2_GetActorLocation`) (`self.K2_GetActorLocation` (`self.Player`)))) 250.0)
      (set `self.Pos` (`self.K2_GetActorLocation`))
      (`self.K2_SetActorLocation` (`KismetMathLibrary.MakeVector` (+ 0.5 _pos_x) _pos_y _pos_z))
      (if (< (+ _startpos_x 130.0) _pos_x_2)
        (`self.K2_SetActorLocation` (+ (`self.StartPos`) (130.0 0.0 0.0)))))))

(fn `UserConstructionScript`)