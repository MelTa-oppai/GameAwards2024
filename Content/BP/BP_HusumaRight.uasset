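; Right-hand fusuma (Japanese sliding door) actor that slides open along Y in small steps each time HusumaR is called.
; After ReleasedF clears the key flag, Tick runs a per-frame countdown, then steps the mesh back to its start via TimelineFinished, with no actual Timeline.
; The open-limit check tests X although the door moves on Y.
; The key-prompt widget logic is unconnected and never runs.
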(event `self.ReceiveBeginPlay`
  (bind _output_get (set `self.Pos` (`self.K2_GetActorLocation`)))
  (set `self.StartPos` _output_get)
  (set `self.Player` (`GameplayStatics.GetPlayerCharacter` 0)))

(event `HusumaR`
  (bind (_pos_x _pos_y _pos_z) (`KismetMathLibrary.BreakVector` (`self.Pos`)))
  (bind _startpos_x (`KismetMathLibrary.BreakVector` (`self.StartPos`)))
  (bind _pos_x_2 (`KismetMathLibrary.BreakVector` (`self.Pos`)))
  (set `self.KeyPress` true)
  (set `self.Pos` (`self.K2_GetActorLocation`))
  (`self.K2_SetActorLocation` (`KismetMathLibrary.MakeVector` _pos_x (+ 0.5 _pos_y) _pos_z))
  (set `self.MovedHusuma` true)
  (if (< (+ _startpos_x 30.0) _pos_x_2)
    (`self.K2_SetActorLocation` (+ (`self.StartPos`) (130.0 0.0 0.0)))))

(event `ReleasedF`
  (set `self.KeyPress` false))

(event `self.ReceiveTick`
  (params (DeltaSeconds :type "Float (single-precision)"))
  (if (`self.KeyPress`)
    _
    (elif (`self.MovedHusuma`)
      (bind _output_get (set `self.CloseTime` (+ (`self.CloseTime`) -0.01)))
      (if (<= _output_get 0.0)
        (`self.TimelineFinished`)))))

(event `TimelineFinished`
  (bind (_pos_x _pos_y _pos_z) (`KismetMathLibrary.BreakVector` (`self.Pos`)))
  (bind (_pos_x_2 _pos_y_2) (`KismetMathLibrary.BreakVector` (`self.Pos`)))
  (bind (_startpos_x _startpos_y) (`KismetMathLibrary.BreakVector` (`self.StartPos`)))
  (bind _output_get (set `self.Pos` (`KismetMathLibrary.MakeVector` _pos_x (+ _pos_y -4.0) _pos_z)))
  (if (<= _pos_y_2 _startpos_y)
    ;[1 1 1] 初期化
    (set `self.MovedHusuma` false)
    (set `self.CloseTime` 5.0)
    (else
      (`SceneComponent.K2_SetWorldLocation` (`self.StaticMeshComponent`) _output_get false false))))

(fn `UserConstructionScript`)