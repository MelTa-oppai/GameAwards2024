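; BP_PostMaterial is an actor that puts a Noise widget on screen, apparently as a screen overlay effect.
; On BeginPlay it creates the widget, adds it to the viewport and gives it a random render transform angle.
; Every Tick calls PlayAnimation on the widget's Location animation, with no check for whether it is already playing.
; Despite the name, the graph touches no material or post-process settings.
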(event `self.ReceiveBeginPlay`
  (bind _returnvalue (`|CreateWidget` "/Game/UMG/Noise.Noise_C"))
  (bind _output_get (set `self.Noise` _returnvalue))
  (`UserWidget.AddToViewport` _output_get 0)
  (`Widget.SetRenderTransformAngle` (`self.Noise`) (`KismetMathLibrary.Conv_IntToDouble` (`KismetMathLibrary.RandomInteger` 100))))

(event `self.ReceiveTick`
  (params (DeltaSeconds :type "Float (single-precision)"))
  (bind _noise (`self.Noise`))
  (`UserWidget.PlayAnimation` _noise (`/Game/UMG/Noise.location` _noise) 0.0 1 "Forward" 1.0 false))

(fn `UserConstructionScript`)