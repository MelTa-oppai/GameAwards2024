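; BP_Player_Cube is a cube actor that shadows the player character and lets them trigger a pair of Husuma (sliding door) actors.
; Each Tick it copies the player's location and rotation, with a fixed Y offset, yaw turn and scale.
; While F is held and the player is near either HusumaR or HusumaL, it calls the trigger functions on both, repeating every frame.
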(event `self.ReceiveBeginPlay`
  (bind _output_get (set `self.Player` (`GameplayStatics.GetPlayerCharacter` 0)))
  (set `self.PlayerPos` (`self.K2_GetActorLocation` _output_get)))

(event `Key|F`
  (params (Key :type "Key Structure"))
  (:`Pressed`
    (set `self.PressKey` true))
  (:`Released`
    (set `self.PressKey` false)))

(event `self.ReceiveTick`
  (params (DeltaSeconds :type "Float (single-precision)"))
  (bind _husumar (`self.HusumaR`))
  (bind _husumal (`self.HusumaL`))
  (bind _returnvalue (`self.GetTransform` (`self.Player`)))
  (`|ExecutionSequence`
    (:`then_0`
      (bind _output_get (set `self.PlayerPos` (.location _returnvalue)))
      (`self.K2_SetActorTransform` (`KismetMathLibrary.MakeTransform` (`KismetMathLibrary.MakeVector` (.x _output_get) (+ (.y _output_get) -50.0) (.z _output_get)) (`KismetMathLibrary.MakeRotator` (.roll (.rotation _returnvalue)) (.pitch (.rotation _returnvalue)) (+ (.yaw (.rotation _returnvalue)) 90.0)) (0.25 0.55 0.25)))
      (`|ExecutionSequence`
        (:`then_0`
          (if (< (`KismetMathLibrary.VSize` (- (`self.K2_GetActorLocation` (`self.HusumaR`)) (`self.K2_GetActorLocation` (`self.Player`)))) 250.0)
            (if (`self.PressKey`)
              (`/Game/BP/BP_HusumaRight.HusumaR` _husumar)
              (`/Game/BP/BP_HusumaLeft.HusumaL` _husumal))))
        (:`then_1`
          (if (< (`KismetMathLibrary.VSize` (- (`self.K2_GetActorLocation` (`self.HusumaL`)) (`self.K2_GetActorLocation` (`self.Player`)))) 250.0)
            (if (`self.PressKey`)
              (`/Game/BP/BP_HusumaLeft.HusumaL` _husumal)
              (`/Game/BP/BP_HusumaRight.HusumaR` _husumar))))))))

(fn `UserConstructionScript`)